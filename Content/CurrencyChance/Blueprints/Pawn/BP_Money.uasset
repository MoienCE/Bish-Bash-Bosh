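; BP_Money is a clickable money piece in a pair-matching game, initialized with an ID, type, mesh and material.
; It flips back shortly after BeginPlay and shows a hand cursor on hover.
; A click, gated by GameStatus, flips it to the front, reports its ID and binds to the GameMode's equality-check event.
; A match plays a scale timeline, while a mismatch flips it back.
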(event Custom|Flip%20Back
  (bind _body (Variables|Default|Getbody))
  (bind _body_2 (Variables|Default|Getbody))
  (bind _relativelocation (Variables|/Script/Engine.SceneComponent|GetRelativeLocation _body))
  (bind _relativelocation_2 (Variables|/Script/Engine.SceneComponent|GetRelativeLocation _body_2))
  ;[0 0 0] Flip BACK, UnFreez
  (Components|MoveComponentTo _body (+ (Math|Vector|MakeVector (.x _relativelocation) (.y _relativelocation) 0.0) (Math|Vector|MakeVector 0.0 0.0 5.0)) "0, 0, 0" true true 0.2 true)
  (Components|MoveComponentTo _body_2 (Math|Vector|MakeVector (.x _relativelocation_2) (.y _relativelocation_2) 0.0) "0, 0, 0" true true 0.15 true)
  (Variables|Default|SetIsFreezed false))

(event Custom|OnEqualityChecked_Event
  (params (Is%20Equal :type Boolean))
  ;[0.1712 0.2781 0.5] Binding to GameMode to tell us what to do accourding to the resault of checking the equality
  (EventDispatchers|UnbindallEventsfromOnEqualityChecked (stale MouseInput|EventActorOnClicked _asbp_game_mode))
  (if Is%20Equal
    ;[0 0.1 0] Equal, Bump, Bye Bye
    (bind _scale_value (Timeline|Timeline PlayFromStart)
      (:Update
        (Transformation|SetRelativeScale3D (Variables|Default|Getbody) (Math|Conversions|ToVector(Float) _scale_value))))
    (else
      ;[0.1667 0 0] NOT Equal (just flip)
      (Variables|Default|SetIsFreezed false)
      (CallFunction|FlipBack))))

(event Custom|Flip%20Front
  (bind _body (Variables|Default|Getbody))
  (bind _body_2 (Variables|Default|Getbody))
  (bind _relativelocation (Variables|/Script/Engine.SceneComponent|GetRelativeLocation _body))
  (bind _relativelocation_2 (Variables|/Script/Engine.SceneComponent|GetRelativeLocation _body_2))
  ;[0 0 0] Flip Front Freez
  (Variables|Default|SetIsFreezed true)
  (Components|MoveComponentTo _body (+ (Math|Vector|MakeVector (.x _relativelocation) (.y _relativelocation) 0.0) (Math|Vector|MakeVector 0.0 0.0 5.0)) "180.000000,0.000000,0.000000" true true 0.2 true)
  (Components|MoveComponentTo _body_2 (+ (Math|Vector|MakeVector (.x _relativelocation_2) (.y _relativelocation_2) 0.0) (Math|Vector|MakeVector 0.0 0.0 1.0)) "180.000000,0.000000,0.000000" true true 0.15 true))

(event EventBeginPlay
  ;[0.3 0.3 0.1] Record PlayerController and GameStatus
  (Utilities|FlowControl|Sequence
    (:then_0
      (Utilities|FlowControl|Delay 2.8)
      (CallFunction|FlipBack))
    (:then_1
      (bind _aspc_default (Utilities|Casting|CastToPC_Default (Game|GetPlayerController 0)))
      (Variables|Default|SetplayerController _aspc_default))
    (:then_2
      (bind _asbp_game_status (Utilities|Casting|CastToBP_GameStatus (Game|GetGameState)))
      (Variables|Default|SetGameStatus _asbp_game_status))))

(event MouseInput|EventActorEndCursorOver
  ;[0.2 0.1 0.2] change mouse icon when mouse is over
  (Variables|/Script/Engine.PlayerController|SetCurrentMouseCursor (Variables|Default|GetplayerController) "Default"))

(event MouseInput|EventActorBeginCursorOver
  ;[0.2 0.1 0.2] change mouse icon when mouse is over
  (Variables|/Script/Engine.PlayerController|SetCurrentMouseCursor (Variables|Default|GetplayerController) "Hand"))

(event MouseInput|EventActorOnClicked
  (params (ButtonPressed :type Key%20Structure :default "None"))
  ;[0.4323 0.4323 0.4323] Clicked on The Money
  (if (not (Variables|/Game/CurrencyChance/Blueprints/FrameWork/BP_GameStatus.BP_GameStatus_C|GetIs%20Found%20Front (Variables|Default|GetGameStatus)))
    (Variables|/Script/Engine.PlayerController|SetCurrentMouseCursor (Variables|Default|GetplayerController) "Default")
    (CallFunction|FlipFront)
    ;[0.2292 0.2292 0.2292] Update GameStatus
    (Default|Update (Variables|Default|GetGameStatus) (Variables|Default|GetID))
    ;[0.1712 0.2781 0.5] Binding to GameMode to tell us what to do accourding to the resault of checking the equality
    (bind _asbp_game_mode (Utilities|Casting|CastToBP_GameMode (Game|GetGameMode)))
    (EventDispatchers|AssignOnEqualityChecked _asbp_game_mode (delegate Custom|OnEqualityChecked_Event))))

(fn ConstructionScript)

(fn GetID
  (return (Variables|Default|GetID)))

(fn Initial
  (params (newID :type Integer) (type :type Integer) (Mesh :type Static%20Mesh%20Object%20Reference) (Material :type Material%20Object%20Reference))
  (bind _sm_money (Variables|Default|GetSM_Money))
  (Variables|Default|SetID newID)
  (Variables|Default|Settype type)
  (Components|StaticMesh|SetStaticMesh _sm_money Mesh)
  (Rendering|Material|SetMaterial _sm_money 0 Material))

(fn GetType
  (return (Variables|Default|Gettype)))