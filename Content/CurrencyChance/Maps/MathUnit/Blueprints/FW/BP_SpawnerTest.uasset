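; BP_SpawnerTest is a grid spawner that fills a four-corner area with evenly spaced BP_Object actors.
; The construction script bilinearly interpolates between points A, B, C and D across Column by Row, lerping along the A-B and C-D edges, then between them.
; It appends each point to Transforms with zero rotation and unit scale, without clearing the array first.
; BeginPlay spawns one BP_Object at each stored transform.
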(event EventBeginPlay
  (for _array_element (Variables|Default|GetTransforms)
    (Game|SpawnActorfromClass "/Game/CurrencyChance/Maps/MathUnit/Blueprints/Env/BP_Object.BP_Object_C" _array_element "Undefined" "MultiplyWithRoot" 0 0)))

(fn ConstructionScript
  (bind _column (Variables|Cards|GetColumn))
  (bind _row (Variables|Cards|GetRow))
  (bind _returnvalue (- _column 1))
  (bind _returnvalue_2 (- _row 1))
  ;[0 0.02604 0.001894] Outer loop
  (for _index (range 0 _returnvalue)
    ;;[0.5898 0.6458 0.4821] FractionX = i / (Column - 1)
    (LocalVariables|SetFractionX%20 (/ (Math|Conversions|ToFloat(Integer) _index) (Math|Conversions|ToFloat(Integer) _returnvalue)))
    ;;[1 0.778 0.7481] From
    (LocalVariables|SetInterpTop%20 (Math|Vector|Lerp(Vector) (Variables|SpawnArea|GetA) (Variables|SpawnArea|GetB) (LocalVariables|GetFractionX%20)))
    ;;[0.6868 0.9801 1] To
    (LocalVariables|SetInterpBottom%20 (Math|Vector|Lerp(Vector) (Variables|SpawnArea|GetC) (Variables|SpawnArea|GetD) (LocalVariables|GetFractionX%20)))
    ;;[0 0.3986 0.4062] Inner Loop
    (for _index_2 (range 0 _returnvalue_2)
      ;;;[0.6614 1 0.655] FractionY = j / (column - 1)
      (bind _output_get (LocalVariables|SetFractionY (/ (Math|Conversions|ToFloat(Integer) _index_2) (Math|Conversions|ToFloat(Integer) _returnvalue_2))))
      ;;;[1 1 0] according to j, where should I put it From Top to Down
      (bind _output_get_2 (LocalVariables|SetFinalLocation (Math|Vector|Lerp(Vector) (LocalVariables|GetInterpTop%20) (LocalVariables|GetInterpBottom%20) _output_get)))
      ;;;[1 0.005426 0] Final Transform
      (Utilities|Array|Add (Variables|Default|GetTransforms) (Math|Transform|MakeTransform _output_get_2)))))