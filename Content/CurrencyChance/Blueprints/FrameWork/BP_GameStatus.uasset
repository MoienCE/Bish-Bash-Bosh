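; BP_GameStatus holds the shared state of a currency card-matching game: cards, flipped flags, guess strike and the player pawn.
; InsertCard registers each card and resets the guess counters.
; Update marks the first flipped card; on the second, it clears the flags, hardcoded to eight entries, and broadcasts OnEqualityChanged with both cards for comparison.
; IncreaseStrike and ResetStrike maintain the strike, with IncreaseStrike also incrementing the flipped count.
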(event EventBeginPlay)

(event EventTick
  (params (DeltaSeconds :type Float%20%28single-precision%29)))

(fn ConstructionScript)

(fn Update
  (params (ID :type Integer))
  (bind _cards (Variables|Default|GetCards))
  ;[0.2 0.12 0.2] Chack if we already have another card flipped
  (Variables|Default|SetIs%20Found%20Front false)
  (bind (_array_element _array_index) (Utilities|Array|ForEachLoopwithBreak (Variables|Default|GetFlipped%20Cards))
    (:LoopBody
      (if _array_element
        (CallFunction|Resetto false)
        (Variables|Default|SetIs%20Found%20Front true)
        (Default|CallOnEqualityChanged (Utilities|Array|Get(acopy) _cards _array_index) (Utilities|Array|Get(acopy) _cards ID))))
    (:Completed
      (if (not (Variables|Default|GetIs%20Found%20Front))
        (Utilities|Array|SetArrayElem (Variables|Default|GetFlipped%20Cards) ID true)))))

(fn Resetto
  (params (New%20Status :type Boolean))
  (Variables|Default|SetFlipped%20Cards (Utilities|Array|MakeArray New%20Status New%20Status New%20Status New%20Status New%20Status New%20Status New%20Status New%20Status)))

(fn InsertCard
  (params (NewCard :type BP%20Money%20Object%20Reference) (Index :type Integer))
  (Utilities|Array|Insert (Variables|Default|GetCards) NewCard Index)
  (Utilities|Array|Add (Variables|Default|GetFlipped%20Cards) false)
  (Variables|Default|SetIs%20Found%20Front false)
  (Variables|Default|SetPrevious%20Guess 3)
  (Variables|Default|SetGuess%20Strike 0)
  (Variables|Default|SetFlipped%20Numbers 0)
  (Math|Integer|IncrementInt (Variables|Default|GetAmount%20Of%20Cards)))

(fn IncreaseStrike
  (Math|Integer|IncrementInt (Variables|Default|GetGuess%20Strike)
    (:%20%20
      (Math|Integer|IncrementInt (Variables|Default|GetFlipped%20Numbers)))))

(fn ResetStrike
  (Variables|Default|SetGuess%20Strike 0))

(fn InsertPlayer
  (params (Player%20Pawn :type BP%20User%20Object%20Reference))
  (Variables|Default|SetPlayerStatus Player%20Pawn))