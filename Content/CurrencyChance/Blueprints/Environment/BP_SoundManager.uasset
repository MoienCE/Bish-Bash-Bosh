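; BP_SoundManager plays the game's intro monologue, cinematic intro audio and countdown sounds in response to BP_GameMode events.
; Its construction script assigns sound variables to six audio components, and BeginPlay binds handlers to the game mode's action, count, reset and view-map events (the last is empty).
; Action plays Arthur's monologue, then the cinematic intro after a delay unless skipped; counting plays three-two-one-beep a second apart.
; Reset sets the skip flag and stops all audio.
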(event Custom|On%20Action_Event
  (Utilities|Arthur))

(event Custom|On%20View%20Map_Event)

(event Custom|Reset_Event
  (Utilities|Pause))

(event Custom|counting
  (Utilities|Count))

(event EventBeginPlay
  (bind _asbp_game_mode (Utilities|Casting|CastToBP_GameMode (Game|GetGameMode))
    (:then
      (EventDispatchers|AssignOnAction _asbp_game_mode (delegate Custom|On%20Action_Event))
      (EventDispatchers|AssignOnViewMap _asbp_game_mode (delegate Custom|On%20View%20Map_Event))
      (EventDispatchers|BindEventtoCountSound _asbp_game_mode (delegate Custom|counting))
      (EventDispatchers|AssignReset _asbp_game_mode (delegate Custom|Reset_Event)))
    (:CastFailed
      (Development|PrintString "Camera Man: Failed to cast Game mode"))))

(fn ConstructionScript
  (Utilities|FlowControl|Sequence
    (:then_0
      (Audio|Components|Audio|SetSound (Variables|Default|GetAC_ArthurMonologue) (Variables|Audios|GetArthurs_Monologue)))
    (:then_1
      (Audio|Components|Audio|SetSound (Variables|Default|GetAC_CinematicIntro) (Variables|Audios|GetCinematic%20Intro)))
    (:then_2
      (Audio|Components|Audio|SetSound (Variables|Default|GetAC_One) (Variables|Audios|GetOne)))
    (:then_3
      (Audio|Components|Audio|SetSound (Variables|Default|GetAC_Two) (Variables|Audios|GetTwo)))
    (:then_4
      (Audio|Components|Audio|SetSound (Variables|Default|GetAC_Three) (Variables|Audios|GetThree)))
    (:then_5
      (Audio|Components|Audio|SetSound (Variables|Default|GetAC_Beep) (Variables|Audios|GetBeep)))))