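; Game mode for a currency card-matching game that runs the round intro, judges flipped pairs and detects the win.
; BeginPlay triggers card spawning, then a timed action, map view and countdown sequence that holds back click input; player reset respawns and jumps to the countdown.
; BP_GameStatus passes two cards for type comparison, with mismatches damaging BP_User.
; CheerUp uses the previous guess to track streaks and fire strike, bullseye or game-won dispatchers.
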(event Custom|OnEqualityChecked_Event
  (params (First%20Money :type BP%20Money%20Object%20Reference) (Second%20Money :type BP%20Money%20Object%20Reference))
  ;[0 0.5312 0.4064] THE CHECK
  (Utilities|Check First%20Money Second%20Money)
  (Utilities|FlowControl|Sequence
    (:then_0
      (CallFunction|CheerUp (Variables|Default|GetId%20Found))
      (Utilities|FlowControl|Delay 0.7)
      (Default|CallOnEqualityChecked (Variables|Default|GetId%20Found))
      (Variables|/Game/CurrencyChance/Blueprints/FrameWork/BP_GameStatus.BP_GameStatus_C|SetIs%20Found%20Front (Variables|Default|GetGameStatus) false))
    (:then_1
      (if (not (Variables|Default|GetId%20Found))
        (Default|Damage (stale EventBeginPlay _asbp_user))))))

(event Custom|Reset_Event
  (Variables|Default|SetIsSkipped true)
  (Default|CallReset)
  (Default|CallSpawn)
  ;[0 0.8 1] Count Down
  (Default|CallCountSound)
  (Utilities|FlowControl|Delay 0.19)
  (Default|CallOnCountDown)
  (Utilities|FlowControl|Delay 3.0)
  (Variables|/Script/Engine.PlayerController|SetbEnableClickEvents (Game|GetPlayerController 0) true))

(event EventBeginPlay
  (bind _returnvalue (Game|GetPlayerController 0))
  (Utilities|FlowControl|Sequence
    (:then_0
      ;[0.05208 0.01823 0] Listen To Game state to pass 2 cards and check them
      (bind _asbp_game_status (Utilities|Casting|CastToBP_GameStatus (Game|GetGameState)))
      (Variables|Default|SetGameStatus _asbp_game_status)
      (bind _asbp_game_status_2 (Utilities|Casting|CastToBP_GameStatus (Game|GetGameState))
        (:then
          (EventDispatchers|AssignOnEqualityChanged _asbp_game_status_2 (delegate Custom|OnEqualityChecked_Event))
          (Default|CallSpawn)
          (Variables|/Script/Engine.PlayerController|SetbEnableClickEvents _returnvalue false)
          ;[0 0.8 1] Sound, Visual, ACTION!
          (Default|CallOnAction)
          (Utilities|FlowControl|Delay 8.6)
          (if (not (Variables|Default|GetIsSkipped))
            ;[0 0.8 1] Smooth show off the map
            (Default|CallOnViewMap)
            (Utilities|FlowControl|Delay 7.0)
            ;[0 0.8 1] Count Down
            (Default|CallCountSound)
            (Utilities|FlowControl|Delay 0.19)
            (Default|CallOnCountDown)
            (Utilities|FlowControl|Delay 3.0)
            (Variables|/Script/Engine.PlayerController|SetbEnableClickEvents _returnvalue true)))
        (:CastFailed
          (Development|PrintString "BP_GameMode: Failed to cast BP_GameState"))))
    (:then_1
      (bind _asbp_user (Utilities|Casting|CastToBP_User (Game|Player|GetPlayerPawn 0)))
      (EventDispatchers|AssignReset _asbp_user (delegate Custom|Reset_Event))
      (Default|InsertPlayer _asbp_game_status _asbp_user))))

(fn ConstructionScript)

(fn CheerUp
  (params (equality :type Boolean))
  (bind _gamestatus (Variables|Default|GetGameStatus))
  (bind _gamestatus_2 (Variables|Default|GetGameStatus))
  (bind _gamestatus_3 (Variables|Default|GetGameStatus))
  (bind _gamestatus_4 (Variables|Default|GetGameStatus))
  (bind _output_get (LocalVariables|SetGuess%20Resault equality))
  (if (== (+ (Variables|/Game/CurrencyChance/Blueprints/FrameWork/BP_GameStatus.BP_GameStatus_C|GetFlipped%20Numbers _gamestatus_3) 1) (/ (Variables|/Game/CurrencyChance/Blueprints/FrameWork/BP_GameStatus.BP_GameStatus_C|GetAmount%20Of%20Cards _gamestatus_3) 2))
    (if _output_get
      (Default|CallGameWon)
      (else
        (if (== 1 (Variables|/Game/CurrencyChance/Blueprints/FrameWork/BP_GameStatus.BP_GameStatus_C|GetPrevious%20Guess (Variables|Default|GetGameStatus))) :!label _label
          (if (LocalVariables|GetGuess%20Resault)
            (Default|IncreaseStrike _gamestatus)
            (Default|CallOnGuessStrike)
            (Development|PrintString "strike")
            (else
              (Default|ResetStrike _gamestatus)
              (Variables|/Game/CurrencyChance/Blueprints/FrameWork/BP_GameStatus.BP_GameStatus_C|SetPrevious%20Guess _gamestatus 0)))
          (elif (== (Variables|/Game/CurrencyChance/Blueprints/FrameWork/BP_GameStatus.BP_GameStatus_C|GetPrevious%20Guess (Variables|Default|GetGameStatus)) 0)
            (if (LocalVariables|GetGuess%20Resault)
              (Default|IncreaseStrike _gamestatus_2)
              (Variables|/Game/CurrencyChance/Blueprints/FrameWork/BP_GameStatus.BP_GameStatus_C|SetPrevious%20Guess _gamestatus_2 1)
              (else
                (Default|ResetStrike _gamestatus_2)))
            (elif (== (Variables|/Game/CurrencyChance/Blueprints/FrameWork/BP_GameStatus.BP_GameStatus_C|GetPrevious%20Guess (Variables|Default|GetGameStatus)) 3)
              (if (LocalVariables|GetGuess%20Resault)
                (Default|IncreaseStrike _gamestatus_4)
                (Variables|/Game/CurrencyChance/Blueprints/FrameWork/BP_GameStatus.BP_GameStatus_C|SetPrevious%20Guess _gamestatus_4 1)
                (Default|CallOnBullseye)
                (Development|PrintString "bullseye")
                (else
                  (Default|ResetStrike _gamestatus_4)
                  (Variables|/Game/CurrencyChance/Blueprints/FrameWork/BP_GameStatus.BP_GameStatus_C|SetPrevious%20Guess _gamestatus_4 0))))))))
    (else
      (goto _label))))