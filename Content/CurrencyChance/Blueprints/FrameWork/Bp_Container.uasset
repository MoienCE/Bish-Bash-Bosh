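; Board spawner for a money-card game that lays out a shuffled grid of paired BP_Money cards.
; When the game mode's OnCountDown event fires, it rebuilds the transform and type lists and replaces all existing money actors.
; Grid positions come from bilinear interpolation between four corner points over NRow by NColumn.
; Each new card gets an ID, type, mesh and per-type material, then registers with BP_GameStatus.
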(event Custom|Spawn_Event
  (CallFunction|GenerateTransforms)
  (CallFunction|GenerateTypes)
  ;[0 0 0] DeSpawn All The Money
  (bind _outactors (Actor|GetAllActorsOfClass "/Game/CurrencyChance/Blueprints/Pawn/BP_Money.BP_Money_C"))
  (for _array_element _outactors
    (Actor|DestroyActor _array_element))
  ;[0 0.03646 0.01455] ReSpawning process: Spawn & Assign ID
  (for _index (range 0 (Utilities|Array|Length (Variables|Default|GetTypes)))
    (bind _returnvalue (Game|SpawnActorfromClass "/Game/CurrencyChance/Blueprints/Pawn/BP_Money.BP_Money_C" (Utilities|Array|Get(acopy) (Variables|Default|Gettransforms) _index) "Undefined" "MultiplyWithRoot" 0 0))
    (Default|Initial _returnvalue _index (Utilities|Array|Get(acopy) (Variables|Default|GetTypes) _index) (Variables|Mesh|GetMoneyMesh) (Utilities|Array|Get(acopy) (Variables|Materials|GetMaterials) (Utilities|Array|Get(acopy) (Variables|Default|GetTypes) _index)))
    (bind _asbp_game_status (Utilities|GetBPGameStatus))
    (Default|InsertCard _asbp_game_status _returnvalue _index)))

(event EventBeginPlay
  (bind _asbp_game_mode (Utilities|Casting|CastToBP_GameMode (Game|GetGameMode)))
  (EventDispatchers|BindEventtoOnCountDown _asbp_game_mode (delegate Custom|Spawn_Event)))

(fn ConstructionScript)

(fn GenerateTypes
  (bind _types (Variables|Default|GetTypes))
  (Utilities|Array|Clear _types)
  (for _index (range 0 (/ (- (* (Variables|CardNumbers|GetN_Row) (Variables|CardNumbers|GetN_Column)) 1) 2))
    (Utilities|Array|Add _types _index)
    (Utilities|Array|Add _types _index))
  (Utilities|Array|Shuffle _types)
  (return))

(fn GenerateTransforms
  (bind _n_column (Variables|CardNumbers|GetN_Column))
  (bind _n_row (Variables|CardNumbers|GetN_Row))
  (bind _returnvalue (- _n_column 1))
  (bind _returnvalue_2 (- _n_row 1))
  (Utilities|Array|Clear (Variables|Default|Gettransforms))
  ;[0 0.151 0] Outer Loop
  (for _index (range 0 _returnvalue)
    ;;[0.6047 1 0.5807] FractionX = i / (column-1)
    (LocalVariables|SetFractionX (/ (Math|Conversions|ToFloat(Integer) _index) (Math|Conversions|ToFloat(Integer) _returnvalue)))
    ;;[1 0.7344 0.9195] From
    (LocalVariables|SetInterTop (Math|Vector|Lerp(Vector) (Variables|SpawningArea|GetA) (Variables|SpawningArea|GetB) (LocalVariables|GetFractionX)))
    ;;[0.6665 0.7851 1] To
    (LocalVariables|SetInterBottom (Math|Vector|Lerp(Vector) (Variables|SpawningArea|GetC) (Variables|SpawningArea|GetD) (LocalVariables|GetFractionX)))
    ;;[0.1535 0.6736 0.7188] Inner Loop
    (for _index_2 (range 0 _returnvalue_2)
      ;;;[0.6356 1 0.6414] FractionY = j / (Row-1)
      (LocalVariables|SetFractionY (/ (Math|Conversions|ToFloat(Integer) _index_2) (Math|Conversions|ToFloat(Integer) _returnvalue_2)))
      ;;;[1 1 0] According to j, where should I put it From Top to Down
      (bind _output_get (LocalVariables|SetFinalLocation (Math|Vector|Lerp(Vector) (LocalVariables|GetInterTop) (LocalVariables|GetInterBottom) (LocalVariables|GetFractionY))))
      ;;;[1 0 0] Final Transform
      (Utilities|Array|Add (Variables|Default|Gettransforms) (Math|Transform|MakeTransform _output_get)))))