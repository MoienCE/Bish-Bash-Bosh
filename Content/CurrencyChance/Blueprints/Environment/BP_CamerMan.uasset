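; BP_CamerMan is the level's camera actor, which becomes the player's view target on BeginPlay and stages shots for game phases.
; It binds to BP_GameMode's Action, View Map and Count Down events, each triggering its own shot.
; Each shot snaps the camera to a hardcoded transform; Count Down and View Map then ease it along with MoveComponentTo, while Action stays static.
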(event Custom|On%20Action_Event
  (Utilities|SetUp))

(event Custom|On%20View%20Map_Event
  (Utilities|ViewMap))

(event Custom|On%20Count%20Down_Event
  (Utilities|CountDown))

(event EventBeginPlay
  (Game|Player|SetViewTargetwithBlend (Game|GetPlayerController 0) self 0.0 "VTBlend_Linear" 0.0 false)
  (bind _asbp_game_mode (Utilities|Casting|CastToBP_GameMode (Game|GetGameMode))
    (:then
      (EventDispatchers|AssignOnAction _asbp_game_mode (delegate Custom|On%20Action_Event))
      (EventDispatchers|AssignOnViewMap _asbp_game_mode (delegate Custom|On%20View%20Map_Event))
      (EventDispatchers|AssignOnCountDown _asbp_game_mode (delegate Custom|On%20Count%20Down_Event)))
    (:CastFailed
      (Development|PrintString "Camera Man: Failed to cast Game mode"))))

(fn ConstructionScript)