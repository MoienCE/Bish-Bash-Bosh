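; BP_User is the player pawn, tracking Health and announcing damage, death and reset through event dispatchers.
; On BeginPlay it caches the PC_Default controller and adds the default Enhanced Input mapping context.
; Damage broadcasts current Health before decrementing it, then at zero disables mouse events and broadcasts death.
; The skip input broadcasts a reset and restores Health, with a DoOnce and Delay acting as a cooldown.
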(event Input|EnhancedActionEvents|EnhancedInputActionIA_Skip
  (params (ActionValue :type Boolean) (ElapsedSeconds :type Float%20%28double-precision%29) (TriggeredSeconds :type Float%20%28double-precision%29) (InputAction :type Input%20Action%20Object%20Reference :default "/Game/CurrencyChance/Input/IA_Skip.IA_Skip"))
  (Utilities|FlowControl|DoOnce false :!label _label
    (:Completed
      (Default|CallReset)
      (Variables|Default|SetHealth 4)
      (Utilities|FlowControl|Delay 4.0)
      (goto _label Reset))))

(event EventBeginPlay
  ;[0.09375 0.05908 0.08104] Get Enhanced Input
  (bind _aspc_default (Utilities|Casting|CastToPC_Default (Game|GetPlayerController 0))
    (:then
      (Variables|Default|SetAs%20PC%20Default _aspc_default)
      (Utilities|IsValid (PlayerController|LocalPlayerSubsystems|GetEnhancedInputLocalPlayerSubsystem _aspc_default)
        (:Is%20Valid
          (Input|AddMappingContext (PlayerController|LocalPlayerSubsystems|GetEnhancedInputLocalPlayerSubsystem _aspc_default) "/Game/CurrencyChance/Input/IMC_Default.IMC_Default" 0 "(bIgnoreAllPressedKeysUntilRelease=True,bForceImmediately=False,bNotifyUserSettings=False)"))
        (:Is%20Not%20Valid
          (Development|PrintString "BP_User: Enhanced Input is not valid"))))
    (:CastFailed
      (Development|PrintString "BP_User: Failed to cast to PC_Default"))))

(fn ConstructionScript)

(fn Damage
  (Default|CallOnDamaged (Variables|Default|GetHealth))
  (bind _result (Math|Integer|DecrementInt (Variables|Default|GetHealth))
    (:%20%20
      (if (== _result 0)
        (Default|EnableMouseEvents (Variables|Default|GetAs%20PC%20Default) false)
        (Default|CallOnDies)))))