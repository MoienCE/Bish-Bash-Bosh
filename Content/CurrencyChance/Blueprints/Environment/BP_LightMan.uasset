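; BP_LightMan is an environment light that changes its spotlight color to signal game phases such as map viewing and the countdown.
; On BeginPlay it binds to the view-map and countdown dispatchers on BP_GameMode, printing an error if the cast fails.
; Map viewing turns the light yellow.
; The countdown steps through red, yellow and green with delays, then a timeline fades green to white, as its name indicates.
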(event Custom|On%20View%20Map_Event
  (Rendering|Components|Light|SetLightColor (Variables|Default|GetSpotLight) "(R=1.000000,G=1.000000,B=0.000000,A=1.000000)" true))

(event Custom|On%20Count%20Down_Event
  (|Countdown))

(event EventBeginPlay
  (bind _asbp_game_mode (Utilities|Casting|CastToBP_GameMode (Game|GetGameMode))
    (:then
      (EventDispatchers|AssignOnViewMap _asbp_game_mode (delegate Custom|On%20View%20Map_Event))
      (EventDispatchers|BindEventtoOnCountDown _asbp_game_mode (delegate Custom|On%20Count%20Down_Event)))
    (:CastFailed
      (Development|PrintString "BP_LightMan: Failed to cast BP_GameMode"))))

(event Collision|EventActorBeginOverlap
  (params (OtherActor :type Actor%20Object%20Reference)))

(event EventTick
  (params (DeltaSeconds :type Float%20%28single-precision%29)))

(fn ConstructionScript)